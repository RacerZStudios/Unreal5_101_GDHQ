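; Placement preview actor that shows a static mesh and signals through its material whether a spawn spot is valid.
; Separate events set the preview mesh's collision mode and swap its static mesh.
; A material event picks a valid or invalid material from a spawn-validity flag, and another restores a default material from an indexed array.
; All material changes affect only the first slot.
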(event Custom|SwitchPreviewMesh
  (Components|StaticMesh|SetStaticMesh (Variables|Default|GetSM_PreviewMesh) (Variables|Default|GetNewMesh)))

(event Custom|SwitchMaterial
  (if (Variables|Default|GetIsValidSpawn)
    (Rendering|Material|SetMaterial (Variables|Default|GetSM_PreviewMesh) 0 (Variables|Default|GetValidMaterial))
    (else
      (Rendering|Material|SetMaterial (Variables|Default|GetSM_PreviewMesh) 0 (Variables|Default|GetInvalidMaterial)))))

(event Custom|SwitchCollisionType
  (Collision|SetCollisionEnabled (Variables|Default|GetSM_PreviewMesh) (Variables|Default|GetCollisionType)))

(event Custom|SetDefaultMaterial
  (Rendering|Material|SetMaterial (Variables|Default|GetSM_PreviewMesh) 0 (Utilities|Array|Get(acopy) (Variables|Default|GetDefaultMaterials) (Variables|Default|GetDefaultMaterialIndex))))

(fn ConstructionScript)